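; BP_GraphNode is a node actor in a BP_Graph, displayed as a sprite icon for a Person, Event, State or Place.
; HideOrShow hides the node unless it is Seeable, otherwise sets its icon by Type and fades it to near-transparent unless Nearby.
; Hover and Unhover toggle the PS component of each connected edge, looked up by EdgeIds in the attach-parent BP_Graph's Edges map.
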(event EventTick
  (params (DeltaSeconds :type Float%20%28single-precision%29)))

(fn ConstructionScript)

(fn SetIcon
  (bind _spritecomponent (Variables|Default|GetSpriteComponent))
  (switch string (Variables|Default|GetType)
    (:person
      (Rendering|Components|Sprite|SetSprite _spritecomponent "/Game/Sprites/person_Sprite.person_Sprite"))
    (:event
      (Rendering|Components|Sprite|SetSprite _spritecomponent "/Game/Sprites/event_Sprite.event_Sprite"))
    (:state
      (Rendering|Components|Sprite|SetSprite _spritecomponent "/Game/Sprites/state_Sprite.state_Sprite"))
    (:place
      (Rendering|Components|Sprite|SetSprite _spritecomponent "/Game/Sprites/place_Sprite.place_Sprite"))))

(fn HideorShow
  (bind _spritecomponent (Variables|Default|GetSpriteComponent))
  (if (Variables|Default|GetSeeable)
    (Rendering|SetActorHiddenInGame false)
    (CallFunction|SetIcon)
    (if (Variables|Default|GetNearby)
      (Sprite|SetSpriteColor _spritecomponent "(R=1.000000,G=1.000000,B=1.000000,A=1.000000)")
      (else
        (Sprite|SetSpriteColor _spritecomponent "(R=1.000000,G=1.000000,B=1.000000,A=0.100000)")))
    (else
      (Rendering|SetActorHiddenInGame true)
      (Rendering|Components|Sprite|SetSprite (Variables|Default|GetSpriteComponent) 0))))

(fn Hover
  (Utilities|FlowControl|Sequence
    (:then_0
      (if true
        _))
    (:then_1
      (if (> (Utilities|Set|Length (Variables|Default|GetEdgeIds)) 0)
        (bind _asbp_graph (Utilities|Casting|CastToBP_Graph (Actor|GetAttachParentActor)))
        (bind _result (Utilities|Set|ToArray (Variables|Default|GetEdgeIds)))
        (for _array_element _result
          (Rendering|SetVisibility (Variables|/Script/History.GraphEdge|GetPS (.Value (Utilities|Map|Find (Variables|/Script/History.Graph|GetEdges _asbp_graph) _array_element))) true false))))))

(fn Unhover
  (Utilities|FlowControl|Sequence
    (:then_0
      (if true
        _))
    (:then_1
      (if (> (Utilities|Set|Length (Variables|Default|GetEdgeIds)) 0)
        (bind _result (Utilities|Set|ToArray (Variables|Default|GetEdgeIds)))
        (for _array_element _result
          (bind _asbp_graph (Utilities|Casting|CastToBP_Graph (Actor|GetAttachParentActor)))
          (Rendering|SetVisibility (Variables|/Script/History.GraphEdge|GetPS (.Value (Utilities|Map|Find (Variables|/Script/History.Graph|GetEdges _asbp_graph) _array_element))) false false))))))