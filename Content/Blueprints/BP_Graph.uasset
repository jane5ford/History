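; BP_Graph builds a node-and-edge graph in the world on BeginPlay.
; It spawns nodes from the GraphInfo DataTable and sets their icons, then spawns edges linking node IDs from AdjancyList, storing both in index-keyed maps.
; A final hardcoded loop spawns placeholder "Person" nodes from ID 151 to 10000, apparently for load testing, storing each under key 0.
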(event EventBeginPlay
  (Utilities|FlowControl|Sequence
    (:then_0
      ;[1 1 1] Read DataTable for Spawn NodeBP
      (bind _outrownames (DataTable|GetDataTableRowNames "/Game/Data/GraphInfo.GraphInfo"))
      (Variables|Default|SetNodesCount 10000)
      (for (_array_element _array_index) _outrownames
        (bind _returnvalue (Utilities|GetDataTableRow "/Game/Data/GraphInfo.GraphInfo" _array_element)
          (:then
            (bind _returnvalue_2 (Class|Graph|SpawnNodeBP _array_index (.type (Utilities|Struct|Breakinfo_GraphNodes _returnvalue)) (.text (Utilities|Struct|Breakinfo_GraphNodes _returnvalue)) (.date (Utilities|Struct|Breakinfo_GraphNodes _returnvalue))))
            (Utilities|Map|Add (Variables|Default|GetNodes) _array_index _returnvalue_2)
            (bind _asbp_graph_node (Utilities|Casting|CastToBP_GraphNode _returnvalue_2))
            (Default|SetIcon _asbp_graph_node)))))
    (:then_1
      ;[1 1 1] Read DataTable for Spawn Edge
      (bind _outrownames_2 (DataTable|GetDataTableRowNames "/Game/Data/AdjancyList.AdjancyList"))
      (for (_array_element_2 _array_index_2) _outrownames_2
        (bind _returnvalue_3 (Utilities|GetDataTableRow "/Game/Data/AdjancyList.AdjancyList" _array_element_2)
          (:then
            (bind _returnvalue_4 (Class|Graph|SpawnEdge _array_index_2 (.NodeA (Utilities|Struct|Breakinfo_GraphEdges _returnvalue_3)) (.NodeB (Utilities|Struct|Breakinfo_GraphEdges _returnvalue_3))))
            (Utilities|Map|Add (Variables|Default|GetEdges) _array_index_2 _returnvalue_4)))))
    (:then_2
      (for _index (range 151 (Variables|Default|GetNodesCount))
        (bind _returnvalue_5 (Class|Graph|SpawnNodeBP _index "Person" "Text" "Date"))
        (Utilities|Map|Add (Variables|Default|GetNodes) 0 _returnvalue_5)))))

(event Collision|EventActorBeginOverlap
  (params (OtherActor :type Actor%20Object%20Reference)))

(event EventTick
  (params (DeltaSeconds :type Float%20%28single-precision%29)))

(fn ConstructionScript)